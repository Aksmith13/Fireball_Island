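; Fireable is a projectile actor that kills enemies and leaves a pickup where they were.
; Each Tick teleports it a fixed step along world +X without sweep or delta-time scaling, so its speed depends on frame rate.
; On overlap with an Enemy, it destroys that enemy and itself, then spawns a Pickup at the enemy's location.
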(event EventActorBeginOverlap
  (params (OtherActor :type Actor%20Object%20Reference))
  ;[1 1 1] When a fireable hits an enemy, destroy the enemy and the fireable
  (bind _asenemy_c (Utilities|Casting|CastToEnemy OtherActor))
  (Actor|DestroyActor _asenemy_c)
  (Actor|DestroyActor)
  ;[1 1 1] Spawn pickup
  (Game|SpawnActorfromClass "/Game/Blueprints/Pickup.Pickup_C" (Math|Conversions|ToTransform(Vector) (Transformation|GetActorLocation _asenemy_c)) false 0))

(event EventTick
  (params (DeltaSeconds :type Float%20%28single-precision%29))
  (bind _returnvalue (Transformation|GetActorLocation))
  (bind (_x _y _z) (Math|Vector|BreakVector _returnvalue))
  ;[1 1 1] Move Firebale
  (Transformation|SetActorLocation (Math|Vector|MakeVector (+ _x 5e+01) _y _z) false))

(fn ConstructionScript)